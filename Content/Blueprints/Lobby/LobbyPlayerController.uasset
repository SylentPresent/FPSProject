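; Lobby player controller that owns the client-side lobby UI for a multiplayer session.
; It creates the lobby widget with server name, map, mode and slots, then forwards player list additions, clears and player count updates to it.
; A kick event opens the main menu level and destroys the session, and a loading screen event swaps the lobby widget for a loading widget.
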(event `AddPlayer`
  (params (`Fail?` :type Boolean) (Player :type Text) (Avatar :type "Texture2D Object Reference") (PlayerIndex :type Integer))
  ;[1 1 1] AddPlayerToList
  (`/Game/UMG/MainMenu/MultiPlayer/LobbyWB.AddPlayerToList` (`self.LobbyWB`) `Fail?` Player Avatar PlayerIndex))

(event `Kick`
  ;[1 1 1] Kick
  (`GameplayStatics.OpenLevel` "MainMenuLevel")
  (`DestroySessionCallbackProxy.DestroySession` self))

(event `ClearPlayerList`
  ;[1 1 1] ClearList
  (`/Game/UMG/MainMenu/MultiPlayer/LobbyWB.ClearPlayerList` (`self.LobbyWB`)))

(event `AddLobbyWB`
  (params (ServerName :type String) (ServerMap :type String) (ServerMode :type String) (ServerSlots :type Integer))
  (set `self.bShowMouseCursor` true)
  (bind _returnvalue (`|CreateWidget` "/Game/UMG/MainMenu/MultiPlayer/LobbyWB.LobbyWB_C" null (`KismetTextLibrary.Conv_StringToText` ServerName) (`KismetTextLibrary.Conv_StringToText` ServerMap) (`KismetTextLibrary.Conv_StringToText` ServerMode) ServerSlots))
  (bind _output_get (set `self.LobbyWB` _returnvalue))
  (`UserWidget.AddToViewport` _output_get 1))

(event `UpdateNumberOfPlayers`
  (params (currentPlayers :type Integer))
  (set `/Game/UMG/MainMenu/MultiPlayer/LobbyWB.currentPlayers` currentPlayers (`self.LobbyWB`)))

(event `LoadingScreen`
  (`Widget.RemoveFromParent` (`self.LobbyWB`))
  (bind _returnvalue (`|CreateWidget` "/Game/UMG/LoadingScreen.LoadingScreen_C" self))
  (`UserWidget.AddToViewport` _returnvalue 0))

(fn `UserConstructionScript`)