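; Lobby game mode that tracks connected player controllers and gives each joiner a lobby widget with the server settings from the game instance.
; UpdateServer rebuilds every client's player list with names, Steam avatars and player count after logins and logouts.
; It also kicks by index and server-travels to the chosen map, defaulting to Map1.
; OnLogout's controller match is unwired, so removal uses the loop's final index rather than the leaver's.
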(event `UpdateServer`
  ;[1 1 1] UpdateServer
  (for _array_element (`self.AllPCs`)
    (bind _aslobby_player_controller (cast `/Game/Blueprints/Lobby/LobbyPlayerController` _array_element))
    (`/Game/Blueprints/Lobby/LobbyPlayerController.ClearPlayerList` _aslobby_player_controller)
    (for (_array_element_2 _array_index) (`self.AllPCs`)
      (bind _returnvalue (`AdvancedSteamFriendsLibrary.GetSteamFriendAvatar` (`AdvancedSessionsLibrary.GetUniqueNetID` _array_element_2) "SteamAvatar_Small")
        (:`OnSuccess`
          (set `self.Fail` false))
        (:`AsyncLoading`
          (set `self.Fail` true))
        (:`OnFailure`
          (set `self.Fail` true)))
      (`/Game/Blueprints/Lobby/LobbyPlayerController.AddPlayer` _aslobby_player_controller (`self.Fail`) (`KismetTextLibrary.Conv_StringToText` (`AdvancedSessionsLibrary.GetPlayerName` _array_element_2)) _returnvalue _array_index)))
  (for _array_element_3 (`self.AllPCs`)
    (bind _aslobby_player_controller_2 (cast `/Game/Blueprints/Lobby/LobbyPlayerController` _array_element_3))
    (`/Game/Blueprints/Lobby/LobbyPlayerController.UpdateNumberOfPlayers` _aslobby_player_controller_2 (`KismetArrayLibrary.Array_Length` (`self.AllPCs`)))))

(event `KickPlayer`
  (params (Index :type Integer))
  (bind _aslobby_player_controller (cast `/Game/Blueprints/Lobby/LobbyPlayerController` (`|GetArrayItem` (`self.AllPCs`) Index)))
  (`/Game/Blueprints/Lobby/LobbyPlayerController.Kick` _aslobby_player_controller))

(event `self.K2_PostLogin`
  (params (NewPlayer :type "PlayerController Object Reference"))
  (`/Engine/EditorBlueprintResources/ActorMacros.Switch Has Authority`
    (:`Authority`
      (`KismetArrayLibrary.Array_Add` (`self.AllPCs`) NewPlayer)
      (bind _asmy_game_instace (cast `/Game/Blueprints/MyGameInstace` (`GameplayStatics.GetGameInstance`)))
      (set `self.ServerName` (`/Game/Blueprints/MyGameInstace.ServerName` _asmy_game_instace))
      (set `self.ServerMap` (`/Game/Blueprints/MyGameInstace.ServerMap` _asmy_game_instace))
      (set `self.ServerMode` (`/Game/Blueprints/MyGameInstace.ServerMode` _asmy_game_instace))
      (set `self.ServerSlots` (`/Game/Blueprints/MyGameInstace.ServerSlots` _asmy_game_instace))
      (bind _aslobby_player_controller (cast `/Game/Blueprints/Lobby/LobbyPlayerController` NewPlayer))
      (`/Game/Blueprints/Lobby/LobbyPlayerController.AddLobbyWB` _aslobby_player_controller (`self.ServerName`) (`self.ServerMap`) (`self.ServerMode`) (`self.ServerSlots`))
      (`self.UpdateServer`))))

(event `self.K2_OnLogout`
  (params (ExitingController :type "Controller Object Reference"))
  (bind _allpcs (`self.AllPCs`))
  (for (_array_element _array_index) _allpcs
    _)
  (`KismetArrayLibrary.Array_Remove` _allpcs _array_index)
  (`self.UpdateServer`))

(event `JoinGame`
  (bind _returnvalue (`GameplayStatics.GetPlayerController` 0))
  (if (`KismetStringLibrary.EqualEqual_StrStr` (`self.ServerMap`) "Map1")
    (`KismetSystemLibrary.ExecuteConsoleCommand` "servertravel/Game/Maps/Map1" _returnvalue :!label _label)
    (elif (`KismetStringLibrary.EqualEqual_StrStr` (`self.ServerMap`) "Map2")
      (`KismetSystemLibrary.ExecuteConsoleCommand` "servertravel/Game/Worlds/Map2" _returnvalue)
      (elif (`KismetStringLibrary.EqualEqual_StrStr` (`self.ServerMap`) "Map3")
        (`KismetSystemLibrary.ExecuteConsoleCommand` "servertravel/Game/Maps/Map3" _returnvalue)
        (else
          (goto _label)))))
  (bind _asmy_game_instace (cast `/Game/Blueprints/MyGameInstace` (`GameplayStatics.GetGameInstance`)))
  (`/Game/Blueprints/MyGameInstace.JoinGame` _asmy_game_instace))

(fn `UserConstructionScript`)